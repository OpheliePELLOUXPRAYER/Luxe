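; Player controller that assigns one of two Luxe characters to the player and provides the main menu and lobby entry points.
; After a short delay on BeginPlay, it finds both characters and possesses the first if the game state's Host flag is set (then clears it), otherwise the second.
; G and H switch possession between the two.
; StartMenu creates the menu HUD on authority, while Server_HostLobby and Server_JoinLobby forward to LuxeGameInstance.
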(event `self.ReceiveBeginPlay`
  (`KismetSystemLibrary.Delay` 0.5)
  (bind _outactors (`GameplayStatics.GetAllActorsOfClass` "/Game/AnimStarterPack/Ue4ASP_Character_luxe.Ue4ASP_Character_luxe_C"))
  (if (> (`KismetArrayLibrary.Array_Length` _outactors) 0)
    (set `self.Pawn_1` (`KismetArrayLibrary.Array_Get` _outactors))
    (bind _outactors_2 (`GameplayStatics.GetAllActorsOfClass` "/Game/AnimStarterPack/Ue4ASP_Character_luxe2.Ue4ASP_Character_luxe2_C"))
    (if (> (`KismetArrayLibrary.Array_Length` _outactors_2) 0)
      (set `self.Pawn_2` (`KismetArrayLibrary.Array_Get` _outactors_2))
      (bind _asluxe_game_state (cast `/Game/Blueprints/LuxeGameState` (`GameplayStatics.GetGameState`)))
      (if (`/Game/Blueprints/LuxeGameState.Host` _asluxe_game_state)
        (`self.Possess` (`self.Pawn_1`))
        (`KismetSystemLibrary.PrintString` "Setting host")
        (set `/Game/Blueprints/LuxeGameState.Host` false _asluxe_game_state)
        (else
          (`self.Possess` (`self.Pawn_2`))
          (`KismetSystemLibrary.PrintString` "Setting client")))
      (else
        (`KismetSystemLibrary.PrintString` "can't access actor luxe 2")))
    (else
      (`KismetSystemLibrary.PrintString` "Can't access actor luxe1"))))

(event `self.ReceiveTick`
  (params (DeltaSeconds :type "Float (single-precision)")))

(event `Key|G`
  (params (Key :type "Key Structure" :default "AnyKey"))
  (:`Pressed`
    (`self.UnPossess`)
    (`self.Possess` (`self.Pawn_1`))))

(event `Key|H`
  (params (Key :type "Key Structure" :default "AnyKey"))
  (:`Pressed`
    (`self.UnPossess`)
    (`self.Possess` (`self.Pawn_2`))))

(event `Create Client HUD`
  (bind _returnvalue (`|CreateWidget` "/Game/Blueprints/MainMenuWidget.MainMenuWidget_C" self))
  (`UserWidget.AddToViewport` _returnvalue 0)
  (set `self.playerMenu` _returnvalue)
  (`WidgetBlueprintLibrary.SetInputMode_GameAndUIEx` null)
  (set `self.bShowMouseCursor` true))

(event `Server_HostLobby`
  (bind _asluxe_game_instance (cast `/Game/Blueprints/LuxeGameInstance` (`GameplayStatics.GetGameInstance`)))
  (`/Game/Blueprints/LuxeGameInstance.Host Game` _asluxe_game_instance self))

(event `Server_JoinLobby`
  (bind _asluxe_game_instance (cast `/Game/Blueprints/LuxeGameInstance` (`GameplayStatics.GetGameInstance`)))
  (`/Game/Blueprints/LuxeGameInstance.Join Game` _asluxe_game_instance self))

(event `self.ReceiveEndPlay`
  (params (EndPlayReason :type "EEndPlayReason Enum" :default "Destroyed"))
  (`Widget.RemoveFromParent` (`self.playerMenu`)))

(fn `SetPawnReferences`
  (params (pawn1 :type "Pawn Object Reference") (pawn2 :type "Pawn Object Reference"))
  (set `self.Pawn_1` pawn1)
  (set `self.Pawn_2` pawn2))

(fn `StartMenu`
  (`/Engine/EditorBlueprintResources/ActorMacros.Switch Has Authority`
    (:`Authority`
      (`self.Create Client HUD`))))

(fn `UserConstructionScript`)