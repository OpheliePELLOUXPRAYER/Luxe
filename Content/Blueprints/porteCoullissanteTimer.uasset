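; Sliding double door that opens when something overlaps its Box trigger and closes when an overlap ends, with no filter on the overlapping actor.
; BeginPlay stores each door panel's initial world location.
; Separate left and right timelines play on overlap and reverse on exit, adding their vector output to the stored location as a world-space offset.
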(event `self.ReceiveBeginPlay`
  (`|ExecutionSequence`
    (:`then_0`
      (set `self.porte left location init` (`SceneComponent.K2_GetComponentLocation` (`self.LeftDoor`))))
    (:`then_1`
      (set `self.porte right location init` (`SceneComponent.K2_GetComponentLocation` (`self.RightDoor`))))))

(event `self.Box.OnComponentBeginOverlap`
  (params (OtherActor :type "Actor Object Reference") (OtherComp :type "PrimitiveComponent Object Reference") (OtherBodyIndex :type Integer) (bFromSweep :type Boolean) (SweepResult :type "HitResult Structure (by ref)"))
  (`|ExecutionSequence`
    (:`then_0`
      (bind (_direction _porte_location) (`Timeline|Timeline_left` :!label _label)
        (:`Update`
          (`SceneComponent.K2_SetWorldLocation` (`self.LeftDoor`) (+ _porte_location (`self.porte left location init`)) false false))))
    (:`then_1`
      (bind (_direction_2 _porte_location_2) (`Timeline|TimeLine_Right` :!label _label_2)
        (:`Update`
          (`SceneComponent.K2_SetWorldLocation` (`self.RightDoor`) (+ _porte_location_2 (`self.porte right location init`)) false false))))))

(event `self.Box.OnComponentEndOverlap`
  (params (OtherActor :type "Actor Object Reference") (OtherComp :type "PrimitiveComponent Object Reference") (OtherBodyIndex :type Integer))
  (`|ExecutionSequence`
    (:`then_0`
      (goto _label :!via `Reverse`))
    (:`then_1`
      (goto _label_2 :!via `Reverse`))))

(event `/Game/Blueprints/porteCoullissante.ReceiveActorBeginOverlap`
  (params (OtherActor :type "Actor Object Reference")))

(event `self.ReceiveTick`
  (params (DeltaSeconds :type "Float (single-precision)")))

(fn `UserConstructionScript`)