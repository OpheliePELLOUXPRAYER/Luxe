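; BigPorte is a door actor that slides its Porte component right or left and back again.
; BeginPlay caches the component's world location as the rest position.
; GoToRight and GoToLeft each play their own timeline, whose PorteLocation vector is added to or subtracted from that position.
; ReverseRight and ReverseLeft run the timelines backwards; the file contains no trigger logic for these custom events.
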(event `self.ReceiveBeginPlay`
  ;[1 1 1] Init Location
  (set `self.initLocation` (`SceneComponent.K2_GetComponentLocation` (`self.Porte`))))

(event `GoToRight`
  ;[1 1 1] Move Door
  (bind (_direction _portelocation) (`Timeline|Timeline_0` :!label _label)
    (:`Update`
      (`SceneComponent.K2_SetWorldLocation` (`self.Porte`) (+ (`self.initLocation`) _portelocation) false false))))

(event `self.ReceiveActorBeginOverlap`
  (params (OtherActor :type "Actor Object Reference")))

(event `ReverseRight`
  ;[1 1 1] Move Door
  (goto _label :!via `Reverse`))

(event `self.ReceiveTick`
  (params (DeltaSeconds :type "Float (single-precision)")))

(event `GoToLeft`
  ;[1 1 1] Move Door
  (bind (_direction _portelocation) (`Timeline|Timeline_1` :!label _label_2)
    (:`Update`
      (`SceneComponent.K2_SetWorldLocation` (`self.Porte`) (- (`self.initLocation`) _portelocation) false false))))

(event `ReverseLeft`
  ;[1 1 1] Move Door
  (goto _label_2 :!via `Reverse`))

(fn `UserConstructionScript`)