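; InteractionBox is a cube actor the player can drag, rotate and scale when within range.
; Tick checks distance to the player, setting Interactable and swapping the cube to an emissive blue material when near.
; While in range and Selected, it follows the deprojected mouse at a fixed depth.
; Functions step rotation per axis and scale within limits; they and Selected are not driven within this Blueprint.
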(event `self.ReceiveBeginPlay`)

(event `self.ReceiveActorBeginOverlap`
  (params (OtherActor :type "Actor Object Reference")))

(event `self.ReceiveTick`
  (params (DeltaSeconds :type "Float (single-precision)"))
  (bind (_worldlocation _worlddirection) (`PlayerController.DeprojectMousePositionToWorld` (`GameplayStatics.GetPlayerController` 0)))
  ;[1 1 1] Interactable
  (`/Engine/EditorBlueprintResources/StandardMacros.CompareFloat` (`self.GetDistanceTo` (`GameplayStatics.GetPlayerCharacter` 0)) 1000.0
    (:`>`
      (`|ExecutionSequence`
        (:`then_0`
          (set `self.Interactable` false))
        (:`then_1`
          (`PrimitiveComponent.SetMaterial` (`self.Cube`) 0 "/Game/FirstPerson/Meshes/BaseMaterial.BaseMaterial"))))
    (:`<`
      (`|ExecutionSequence`
        (:`then_0`
          (set `self.Interactable` true)
          ;[1 1 1] Move To the mouse position
          (if (`self.Selected`)
            (`self.K2_SetActorLocation` (+ _worldlocation (* _worlddirection 700.0)))))
        (:`then_1`
          (`PrimitiveComponent.SetMaterial` (`self.Cube`) 0 "/Game/Materials/Master_Emissive_blue.Master_Emissive_blue"))))))

(fn `RotationX`
  (`self.SetActorRotation` (`KismetMathLibrary.MakeRotator` (+ (.roll (`SceneComponent.RelativeRotation` (`self.Cube`))) 15.0) (.pitch (`SceneComponent.RelativeRotation` (`self.Cube`))) (.yaw (`SceneComponent.RelativeRotation` (`self.Cube`))))))

(fn `RotationY`
  (`self.SetActorRotation` (`KismetMathLibrary.MakeRotator` (.roll (`SceneComponent.RelativeRotation` (`self.Cube`))) (+ (.pitch (`SceneComponent.RelativeRotation` (`self.Cube`))) 15.0) (.yaw (`SceneComponent.RelativeRotation` (`self.Cube`))))))

(fn `RotationZ`
  (`self.SetActorRotation` (`KismetMathLibrary.MakeRotator` (.roll (`SceneComponent.RelativeRotation` (`self.Cube`))) (.pitch (`SceneComponent.RelativeRotation` (`self.Cube`))) (+ (.yaw (`SceneComponent.RelativeRotation` (`self.Cube`))) 15.0))))

(fn `scale`
  (params (up :type Boolean))
  (bind _cube (`self.Cube`))
  (bind _returnvalue (`SceneComponent.K2_GetComponentScale` _cube))
  (if up
    (if (and (< (.x _returnvalue) 8.0) (< (.y _returnvalue) 8.0) (< (.z _returnvalue) 8.0))
      (`SceneComponent.SetWorldScale3D` _cube (+ _returnvalue 0.2)))
    (elif (and (> (.x _returnvalue) 0.3) (> (.y _returnvalue) 0.3) (> (.z _returnvalue) 0.3))
      (`SceneComponent.SetWorldScale3D` _cube (- _returnvalue 0.2)))))

(fn `UserConstructionScript`)