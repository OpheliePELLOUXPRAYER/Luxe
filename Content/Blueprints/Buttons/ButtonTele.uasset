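; ButtonTele is a pressure-style button that slides a referenced Door sideways while an InteractionBox rests on it.
; On begin overlap it confirms the box's Cube touches the trigger, then calls GoToLeft or GoToRight according to MoveDoorToLeft.
; On end overlap any InteractionBox triggers the matching ReverseRight or ReverseLeft, without the Cube check.
; Debug prints trace the moves, though the begin-overlap message for other actors is never reached.
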(event `self.ButtonTeleBoxCollision.OnComponentBeginOverlap`
  (params (OtherActor :type "Actor Object Reference") (OtherComp :type "PrimitiveComponent Object Reference") (OtherBodyIndex :type Integer) (bFromSweep :type Boolean) (SweepResult :type "HitResult Structure (by ref)"))
  (bind _door (`self.Door`))
  (bind _asinteraction_box (cast `/Game/Blueprints/InteractionBox` OtherActor))
  (if (`PrimitiveComponent.IsOverlappingComponent` (`/Game/Blueprints/InteractionBox.Cube` _asinteraction_box) (`self.ButtonTeleBoxCollision`))
    (if (`self.MoveDoorToLeft`)
      (`/Game/Blueprints/BigPorte.GoToLeft` _door)
      (`KismetSystemLibrary.PrintString` "ButtonTele BeginOverlap : Overlapping Actor goes to left")
      (else
        (`/Game/Blueprints/BigPorte.GoToRight` _door)
        (`KismetSystemLibrary.PrintString` "ButtonTele BeginOverlap : Overlapping Actor goes to right")))))

(event `self.ButtonTeleBoxCollision.OnComponentEndOverlap`
  (params (OtherActor :type "Actor Object Reference") (OtherComp :type "PrimitiveComponent Object Reference") (OtherBodyIndex :type Integer))
  (bind _door (`self.Door`))
  (cast `/Game/Blueprints/InteractionBox` OtherActor
    (:`then`
      (if (`self.MoveDoorToLeft`)
        (`/Game/Blueprints/BigPorte.ReverseRight` _door)
        (`KismetSystemLibrary.PrintString` "ButtonTele EndOverlap : Overlapping Actor goes to right")
        (else
          (`/Game/Blueprints/BigPorte.ReverseLeft` _door)
          (`KismetSystemLibrary.PrintString` "ButtonTele EndOverlap : Overlapping Actor goes to left"))))
    (:`CastFailed`
      (`KismetSystemLibrary.PrintString` "ButtonTele EndOverlap : Overlaping Actor Not a InteractionBox"))))

(fn `UserConstructionScript`)