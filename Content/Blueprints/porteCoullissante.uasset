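; Sliding double door actor that opens when anything begins overlapping its Box trigger, with no logic to close it again.
; LeftDoor and RightDoor are set toward the Left and Right marker positions via VInterpTo, whose zero speed makes them jump straight there.
; Each side has a short Delay and a Gate that closes once its door reaches the marker, though no gate exit logic appears.
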(event `self.ReceiveBeginPlay`)

(event `self.ReceiveActorBeginOverlap`
  (params (OtherActor :type "Actor Object Reference")))

(event `self.Box.OnComponentBeginOverlap`
  (params (OtherActor :type "Actor Object Reference") (OtherComp :type "PrimitiveComponent Object Reference") (OtherBodyIndex :type Integer) (bFromSweep :type Boolean) (SweepResult :type "HitResult Structure (by ref)"))
  (bind _returnvalue (`SceneComponent.K2_GetComponentLocation` (`self.LeftDoor`)))
  (bind _returnvalue_2 (`SceneComponent.K2_GetComponentLocation` (`self.Left`)))
  (bind _returnvalue_3 (`SceneComponent.K2_GetComponentLocation` (`self.RightDoor`)))
  (bind _returnvalue_4 (`SceneComponent.K2_GetComponentLocation` (`self.Right`)))
  (`|ExecutionSequence`
    (:`then_0`
      (`SceneComponent.K2_SetWorldLocation` (`self.LeftDoor`) (`KismetMathLibrary.VInterpTo` _returnvalue _returnvalue_2 (`GameplayStatics.GetWorldDeltaSeconds`) 0.0) false false)
      (`KismetSystemLibrary.Delay` 0.0001)
      (`|ExecutionSequence`
        (:`then_0`
          (`/Engine/EditorBlueprintResources/StandardMacros.Gate` true :!label _label))
        (:`then_1`
          (if (== _returnvalue _returnvalue_2 :`ErrorTolerance` 0.01)
            (`|ExecutionSequence`
              (:`then_0`
                (goto _label :!via `Close`)))))))
    (:`then_1`
      (`SceneComponent.K2_SetWorldLocation` (`self.RightDoor`) (`KismetMathLibrary.VInterpTo` _returnvalue_3 _returnvalue_4 (`GameplayStatics.GetWorldDeltaSeconds`) 0.0) false false)
      (`KismetSystemLibrary.Delay` 0.0001)
      (`|ExecutionSequence`
        (:`then_0`
          (`/Engine/EditorBlueprintResources/StandardMacros.Gate` true :!label _label_2))
        (:`then_1`
          (if (== _returnvalue_3 _returnvalue_4 :`ErrorTolerance` 0.01)
            (`|ExecutionSequence`
              (:`then_0`
                (goto _label_2 :!via `Close`)))))))
    (:`then_2`
      (goto _label :!via `Open`))
    (:`then_3`
      (goto _label_2 :!via `Open`))))

(event `self.ReceiveTick`
  (params (DeltaSeconds :type "Float (single-precision)")))

(fn `UserConstructionScript`)